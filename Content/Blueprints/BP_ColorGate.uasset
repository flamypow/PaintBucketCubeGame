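; BP_ColorGate is a puzzle gate that opens when a BP_ColoringObject carrying the matching color enters its PuzzleVolume.
; The construction script tints both castle doors and the puzzle plate with the material for the Color variable.
; On a match it clears the object's color, marks itself open permanently, and plays a timeline scaled by TimeToComplete that swings both door pivots 90 degrees.
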(event OnComponentBeginOverlap(PuzzleVolume)
  (params (OverlappedComponent :type Primitive%20Component%20Object%20Reference) (OtherActor :type Actor%20Object%20Reference) (OtherComp :type Primitive%20Component%20Object%20Reference) (OtherBodyIndex :type Integer) (bFromSweep :type Boolean) (SweepResult :type Hit%20Result%20Structure%20%28by%20ref%29))
  (if (not (Variables|Default|GetIsDoorOpen))
    (bind _asbp_coloring_object (Utilities|Casting|CastToBP_ColoringObject OtherActor))
    (bind _returncolor (Default|GetColor _asbp_coloring_object))
    (if (Utilities|Enum|Equal(Enum) _returncolor (Variables|Default|GetColor))
      (Variables|Default|SetIsDoorOpen true)
      (Default|ClearColor _asbp_coloring_object)
      (Components|Timeline|SetPlayRate (Variables|Default|GetOpenGateTimeline) (/ 1.0 (Variables|Default|GetTimeToComplete)))
      (bind _gatetrack (Timeline|OpenGateTimeline Play)
        (:Update
          (bind _result (Math|Float|NegateFloat (Math|Float|Lerp 0.0 9e+01 _gatetrack))
            (:%20%20
              (Transformation|SetRelativeRotation (Variables|Default|GetGatePivotL) (Math|Rotator|MakeRotator 0.0 0.0 _result) false false)
              (Transformation|SetRelativeRotation (Variables|Default|GetGatePivotR) (Math|Rotator|MakeRotator 0.0 0.0 (Math|Float|Lerp 0.0 9e+01 _gatetrack)) false false))))))))

(event EventBeginPlay)

(event Collision|EventActorBeginOverlap
  (params (OtherActor :type Actor%20Object%20Reference)))

(event EventTick
  (params (DeltaSeconds :type Float%20%28single-precision%29)))

(fn ConstructionScript
  (switch Utilities|FlowControl|Switch|SwitchonEnumPuzzleColor (Variables|Default|GetColor)
    (:NewEnumerator0
      (Rendering|Material|SetMaterial (Variables|Default|GetSM_Bld_Castle_Door_L) 0 "/Game/Materials/MI_GreenBlock.MI_GreenBlock"))
    (:NewEnumerator1
      (Rendering|Material|SetMaterial (Variables|Default|GetSM_Bld_Castle_Door_L) 0 "/Game/Materials/MI_BlueBlock.MI_BlueBlock"))
    (:NewEnumerator2
      (Rendering|Material|SetMaterial (Variables|Default|GetSM_Bld_Castle_Door_L) 0 "/Game/Materials/MI_RedBlock.MI_RedBlock"))))

(fn OpenGate)