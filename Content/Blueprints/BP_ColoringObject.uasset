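; BP_ColoringObject is an actor with a Cube component whose displayed material follows a stored Color state.
; ChangeColor stores the new value and switches the cube's first material slot between green, blue and red block materials, or base gray for None.
; GetColor returns the stored state, and ClearColor resets it to None through ChangeColor.
; Its event graph and construction script do nothing, so color changes only when these functions are called.
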(event EventBeginPlay)

(event Collision|EventActorBeginOverlap
  (params (OtherActor :type Actor%20Object%20Reference)))

(event EventTick
  (params (DeltaSeconds :type Float%20%28single-precision%29)))

(fn ConstructionScript)

(fn ChangeColor
  (params (NewParam :type EnumPuzzleColor%20Enum :default "NewEnumerator3"))
  (bind _output_get (Variables|Default|SetColor NewParam))
  (switch Utilities|FlowControl|Switch|SwitchonEnumPuzzleColor _output_get
    (:NewEnumerator3
      (Rendering|Material|SetMaterial (Variables|Default|GetCube) 0 "/Engine/TemplateResources/MI_Template_BaseGray.MI_Template_BaseGray"))
    (:NewEnumerator0
      (Rendering|Material|SetMaterial (Variables|Default|GetCube) 0 "/Game/Materials/MI_GreenBlock.MI_GreenBlock"))
    (:NewEnumerator1
      (Rendering|Material|SetMaterial (Variables|Default|GetCube) 0 "/Game/Materials/MI_BlueBlock.MI_BlueBlock"))
    (:NewEnumerator2
      (Rendering|Material|SetMaterial (Variables|Default|GetCube) 0 "/Game/Materials/MI_RedBlock.MI_RedBlock"))))

(fn GetColor
  (return (Variables|Default|GetColor)))

(fn ClearColor
  (Variables|Default|SetColor "NewEnumerator3")
  (CallFunction|ChangeColor "NewEnumerator3"))