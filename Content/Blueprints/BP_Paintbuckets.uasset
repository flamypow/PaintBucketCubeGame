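; BP_Paintbuckets is a colored paint bucket actor that recolors BP_ColoringObject actors that overlap it.
; The construction script sets the Cube's water material instance to green, blue or red based on its Color variable.
; On overlap, it casts the other actor to BP_ColoringObject and passes that Color to its ChangeColor function.
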(event EventBeginPlay)

(event Collision|EventActorBeginOverlap
  (params (OtherActor :type Actor%20Object%20Reference))
  (bind _asbp_coloring_object (Utilities|Casting|CastToBP_ColoringObject OtherActor))
  (Default|ChangeColor _asbp_coloring_object (Variables|Default|GetColor)))

(event EventTick
  (params (DeltaSeconds :type Float%20%28single-precision%29)))

(fn ConstructionScript
  (switch Utilities|FlowControl|Switch|SwitchonEnumPuzzleColor (Variables|Default|GetColor)
    (:NewEnumerator0
      (Rendering|Material|SetMaterial (Variables|Default|GetCube) 0 "/Game/Materials/Water/MI_GreenWater.MI_GreenWater"))
    (:NewEnumerator1
      (Rendering|Material|SetMaterial (Variables|Default|GetCube) 0 "/Game/Materials/Water/MI_BlueWater.MI_BlueWater"))
    (:NewEnumerator2
      (Rendering|Material|SetMaterial (Variables|Default|GetCube) 0 "/Game/Materials/Water/MI_RedWater.MI_RedWater"))))